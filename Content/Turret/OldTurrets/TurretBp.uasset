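; Player-controllable minigun turret that fades in via a dynamic material, then switches to its final material.
; While controlled, Tick interpolates TurretAnim pitch and yaw toward TankState's aim location and mirrors the player's fire input.
; Minigun_2 chains FireGun, which handles fire rate, montage and spread buildup, into ShootBullets line traces.
; Hits spawn effects, push movable components and damage tagged actors, with cosine distance scaling and headshot bonuses for enemies.
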(event Custom|ParticleEffects
  (params (Rotation :type Rotator) (Location :type Vector) (Parent :type Primitive%20Component%20Object%20Reference))
  (bind _returnvalue (Math|Random|RandomFloatinRange 8.0 1e+01))
  (bind (_roll _pitch _yaw) (Math|Rotator|BreakRotator Rotation))
  (bind _bullettracer (Variables|Default|GetBulletTracer))
  (bind _bullettracer_2 (Variables|Default|GetBulletTracer))
  (bind _returnvalue_2 (Transformation|GetWorldLocation _bullettracer_2))
  (bind _returnvalue_3 (- _returnvalue_2 Location))
  (bind _returnvalue_4 (Math|Rotator|MakeRotfromX _returnvalue_3))
  (bind (_roll_2 _pitch_2 _yaw_2) (Math|Rotator|BreakRotator _returnvalue_4))
  (bind _returnvalue_5 (Class|GameplayStatics|SpawnDecalAttached "/Game/RobotChar/Mats/GunDecal_2.GunDecal_2" (Math|Vector|MakeVector 5.0 _returnvalue _returnvalue) Parent "None" Location (Math|Rotator|MakeRotator (Math|Random|RandomFloatinRange 0.0 3.6e+02) (+ _pitch 1.8e+02) _yaw) "KeepWorldPosition" 6e+01))
  (Class|HoverTank|EditDisplaySize (Variables|/Game/Blueprints/TankState.TankState_C|GetPlayer (Variables|Default|GetTankState)) _returnvalue_5 0.0005)
  (Effects|SpawnEmitteratLocation "/Game/RobotChar/Mats/HitEffect.HitEffect" Location Rotation)
  (Transformation|SetWorldRotation _bullettracer (Math|Rotator|MakeRotator _roll_2 (* _pitch_2 -1.0) (+ _yaw_2 1.8e+02)) false true)
  (Components|Activation|SetActive _bullettracer true true)
  (Components|Activation|SetActive (Variables|Default|GetMuzzleFlash) true true))

(event Custom|ShowCantShoot)

(event EventBeginPlay
  (bind _turretmesh (Variables|Default|GetTurretMesh))
  (bind _asturret_anim (Utilities|Casting|CastToTurretAnim (Components|SkeletalMesh|GetAnimInstance (Variables|Default|GetTurretMesh))))
  (bind _output_get (Variables|Default|SetTurretAnim _asturret_anim))
  (Variables|/Game/Turret/OldTurrets/TurretAnim.TurretAnim_C|SetBoneLocation _output_get (Transformation|GetSocketLocation (Variables|Default|GetTurretMesh) "WrongEnd"))
  (Transformation|SetWorldRotation (Variables|Default|GetSpawnPart) "0, 0, 0" false false)
  (bind _astank_state (Utilities|Casting|CastToTankState (Variables|/Script/Engine.Controller|GetPlayerState (Game|GetPlayerController 0))))
  (Variables|Default|SetTankState _astank_state)
  (Rendering|Material|SetMaterial _turretmesh 0 (Variables|Default|GetDynamicMat))
  (Rendering|SetVisibility _turretmesh true false)
  (Utilities|FlowControl|Delay 1.0)
  (Variables|Default|SetEnabled true)
  (Collision|SetCollisionEnabled (Variables|Default|GetTurretMesh) "QueryOnly")
  (Components|Activation|Deactivate (Variables|Default|GetSpawnPart))
  (Development|PrintString "Hello"))

(event EventTick
  (params (DeltaSeconds :type Float%20%28single-precision%29))
  (bind _tankstate (Variables|Default|GetTankState))
  (bind _turretanim (Variables|Default|GetTurretAnim))
  (bind _turretanim_2 (Variables|Default|GetTurretAnim))
  (bind _player (Variables|/Game/Blueprints/TankState.TankState_C|GetPlayer _tankstate))
  (if (== (Variables|Default|GetCurrentFadeValue) 1.0)
    (Utilities|FlowControl|Sequence
      (:then_0
        (if (and (Variables|Default|GetUnderControl) (Variables|Default|GetEnabled))
          (Utilities|FlowControl|Sequence
            (:then_0
              (Variables|/Game/Turret/OldTurrets/TurretAnim.TurretAnim_C|SetPitch _turretanim (.Pitch (Math|Rotator|BreakRotator (Math|Interpolation|RInterpTo (Math|Rotator|MakeRotator 0.0 (Variables|/Game/Turret/OldTurrets/TurretAnim.TurretAnim_C|GetPitch _turretanim_2) (Variables|/Game/Turret/OldTurrets/TurretAnim.TurretAnim_C|GetYaw _turretanim_2)) (Math|Rotator|MakeRotfromX (Math|Vector|Normalize (- (Transformation|GetSocketLocation (Variables|Default|GetTurretMesh) "Turret") (Variables|/Game/Blueprints/TankState.TankState_C|GetAimLocation (Variables|Default|GetTankState))))) DeltaSeconds 6.0))))
              (Variables|/Game/Turret/OldTurrets/TurretAnim.TurretAnim_C|SetYaw _turretanim (.Yaw (Math|Rotator|BreakRotator (Math|Interpolation|RInterpTo (Math|Rotator|MakeRotator 0.0 (Variables|/Game/Turret/OldTurrets/TurretAnim.TurretAnim_C|GetPitch _turretanim_2) (Variables|/Game/Turret/OldTurrets/TurretAnim.TurretAnim_C|GetYaw _turretanim_2)) (Math|Rotator|MakeRotfromX (Math|Vector|Normalize (- (Transformation|GetSocketLocation (Variables|Default|GetTurretMesh) "Turret") (Variables|/Game/Blueprints/TankState.TankState_C|GetAimLocation (Variables|Default|GetTankState))))) DeltaSeconds 6.0))))
              (Utilities|IsValid _player
                (:Is%20Valid
                  (Variables|Default|SetWantToFire (Variables|/Game/RobotChar/Blueprints/RobotPlayer3.RobotPlayer3_C|GetWantToFire _player))
                  (|Minigun_2 DeltaSeconds))))
            (:then_1
              (goto _label Reset)))
          (else
            (Utilities|FlowControl|DoOnce false :!label _label
              (:Completed
                (Animation|Montage|MontageStop (Variables|Default|GetTurretAnim) 0.0 "/Game/Turret/OldTurrets/GunFireMont.GunFireMont"))))))
      (:then_1
        (Utilities|FlowControl|DoOnce false
          (:Completed
            (Utilities|FlowControl|Delay 0.2)
            (Rendering|Material|SetMaterial (Variables|Default|GetTurretMesh) 0 "/Game/Maps/LevelMeshes/Materials/ProtossWalls.ProtossWalls")))))
    (else
      (bind _output_get (Variables|Default|SetCurrentFadeValue (Math|Float|Clamp(Float) (+ (* DeltaSeconds 1.1) (Variables|Default|GetCurrentFadeValue)))))
      (Rendering|Material|SetScalarParameterValue (Variables|Default|GetDynamicMat) "Fade" _output_get :!class /Script/Engine.MaterialInstanceDynamic))))

(event Input|ActionEvents|InputActionFire
  (params (Key :type Key%20Structure :default "AnyKey"))
  (:Pressed
    (Variables|Default|SetWantToFire true))
  (:Released
    (Variables|Default|SetWantToFire false)))

(fn ConstructionScript
  (bind _returnvalue (Rendering|Material|CreateDynamicMaterialInstance "/Game/OtherActors/Assests/FadingTransInst.FadingTransInst" :!class /Script/Engine.KismetMaterialLibrary))
  (bind _output_get (Variables|Default|SetDynamicMat _returnvalue))
  (Rendering|Material|SetMaterial (Variables|Default|GetTurretMesh) 0 _output_get))

(fn RotatorExpand
  (params (Offset :type Float%20%28single-precision%29) (Rotation :type Rotator))
  (bind (_roll _pitch _yaw) (Math|Rotator|BreakRotator Rotation))
  (bind (_x _y _z) (|Change Offset _roll _pitch _yaw))
  (return (Math|Rotator|MakeRotator _x _y _z)))
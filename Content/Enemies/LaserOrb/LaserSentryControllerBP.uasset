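; AI controller for the laser sentry orb that decides when it engages the player.
; On possess it retries until the player's TankState exists, then runs LaserOrbBehaviour and a looping check timer, cleared on unpossess.
; Unless State is 2, each check sets the blackboard State from range and line-of-sight trace, toggling AbortAndReset when the target is visible.
; A lost target is reacquired from the player pawn.
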(event Custom|Check
  (bind _returnvalue (Pawn|GetControlledPawn))
  (bind _returnvalue_2 (Utilities|Name|MakeLiteralName "State"))
  (bind _returnvalue_3 (Utilities|Name|MakeLiteralName "AbortAndReset"))
  (bind _returnvalue_4 (Game|Player|GetPlayerPawn 0))
  (bind _blackboard (Variables|Default|GetBlackboard))
  (bind _blackboard_2 (Variables|Default|GetBlackboard))
  (bind _returnvalue_5 (Transformation|GetActorLocation _returnvalue))
  (if (!= (Class|BlackboardComponent|GetValueasEnum (Variables|Default|GetBlackboard) (Utilities|Name|MakeLiteralName "State")) 2)
    (Utilities|IsValid (Variables|Default|GetAiTarget)
      (:Is%20Valid
        (if (< (Math|Vector|VectorLength (- (Transformation|GetActorLocation (Variables|Default|GetAiTarget)) _returnvalue_5)) (Variables|Default|GetDistance))
          (bind _returnvalue_6 (Collision|LineTraceForObjects _returnvalue_5 (Transformation|GetActorLocation (Variables|Default|GetAiTarget)) (Utilities|Array|MakeArray "ObjectTypeQuery1" "ObjectTypeQuery2") false (Utilities|Array|MakeArray (Variables|Default|GetAiTarget)) "None" true "(R=1.000000,G=0.000000,B=0.000000,A=1.000000)" "(R=0.000000,G=1.000000,B=0.000000,A=1.000000)" 1.0))
          (if _returnvalue_6
            (AI|Components|Blackboard|SetValueasEnum _blackboard _returnvalue_2)
            (else
              (AI|Components|Blackboard|SetValueasEnum _blackboard _returnvalue_2 1)
              (AI|Components|Blackboard|SetValueasBool _blackboard_2 _returnvalue_3 false)
              (AI|Components|Blackboard|SetValueasBool _blackboard_2 _returnvalue_3 true)))
          (else
            (AI|Components|Blackboard|SetValueasEnum (Variables|Default|GetBlackboard) _returnvalue_2))))
      (:Is%20Not%20Valid
        (Utilities|IsValid _returnvalue_4
          (:Is%20Valid
            (bind _output_get (Variables|Default|SetAiTarget _returnvalue_4))
            (AI|Components|Blackboard|SetValueasObject (Variables|Default|GetBlackboard) (Utilities|Name|MakeLiteralName "TargetAct") _output_get)))))))

(event EventBeginPlay)

(event EventOnPossess
  (params (PossessedPawn :type Pawn%20Object%20Reference))
  (bind _returnvalue (Game|GetPlayerController 0))
  (Utilities|IsValid _returnvalue
    (:Is%20Valid
      (Utilities|Casting|CastToTankState (Variables|/Script/Engine.Controller|GetPlayerState _returnvalue) :!label _label
        (:then
          _)
        (:CastFailed
          (Utilities|FlowControl|Delay 0.2 :!label _label_2)
          (goto _label))))
    (:Is%20Not%20Valid
      (goto _label_2)))
  (Variables|Default|SetAiTarget (Game|Player|GetPlayerPawn 0))
  (AI|RunBehaviorTree "/Game/Enemies/LaserOrb/LaserOrbBehaviour.LaserOrbBehaviour")
  (bind _returnvalue_2 (Utilities|Time|SetTimerbyEvent (delegate Custom|Check) 0.5 true))
  (Variables|Default|SetCheckTimer _returnvalue_2))

(event EventOnUnpossess
  (params (UnpossessedPawn :type Pawn%20Object%20Reference))
  (Utilities|Time|ClearandInvalidateTimerbyHandle (Variables|Default|GetCheckTimer)))

(event EventTick
  (params (DeltaSeconds :type Float%20%28single-precision%29)))

(fn ConstructionScript)